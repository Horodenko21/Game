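; Player stats component that tracks health, stamina and mana for BP_ThirdPersonCharacter and drives its HUD bars.
; BeginPlay waits a tick, caches the owning character and fills the bars.
; Decrease functions return true on depletion, Recover functions cap at the maximum, and IncreaseMax functions raise only the maximum.
; Each change pushes a current/max percent to its bar, except DecreaseMana, which divides by MaxHealth instead of MaxMana.
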(event `self.ReceiveBeginPlay`
  (`KismetSystemLibrary.DelayUntilNextTick`)
  (bind _asbp_third_person_character (cast `/Game/ThirdPerson/Blueprints/BP_ThirdPersonCharacter` (`self.GetOwner`)))
  (set `self.PlayerCharacterBP` _asbp_third_person_character)
  (`ProgressBar.SetPercent` (`/Game/Kori/UI/WB_HUD.HealthBar` (`/Game/ThirdPerson/Blueprints/BP_ThirdPersonCharacter.HUDWidget` (`self.PlayerCharacterBP`))) (/ (`self.CurrentHealth`) (`self.MaxHealth`)))
  (`ProgressBar.SetPercent` (`/Game/Kori/UI/WB_HUD.StaminaBar` (`/Game/ThirdPerson/Blueprints/BP_ThirdPersonCharacter.HUDWidget` (`self.PlayerCharacterBP`))) (/ (`self.CurrentStamina`) (`self.MaxStamina`)))
  (`ProgressBar.SetPercent` (`/Game/Kori/UI/WB_HUD.ManaBar` (`/Game/ThirdPerson/Blueprints/BP_ThirdPersonCharacter.HUDWidget` (`self.PlayerCharacterBP`))) (/ (`self.CurrentMana`) (`self.MaxMana`))))

(fn `DecreaseHealth`
  (params (Damage :type "Float (double-precision)"))
  (returns (isDead :type Boolean))
  (if (not (<= (`self.CurrentHealth`) 0.0))
    (bind _output_get (set `self.CurrentHealth` (- (`self.CurrentHealth`) Damage)))
    (`ProgressBar.SetPercent` (`/Game/Kori/UI/WB_HUD.HealthBar` (`/Game/ThirdPerson/Blueprints/BP_ThirdPersonCharacter.HUDWidget` (`self.PlayerCharacterBP`))) (/ _output_get (`self.MaxHealth`)))
    (if (<= (`self.CurrentHealth`) 0.0)
      _
      (else
        (return false))))
  (return true))

(fn `DecreaseMana`
  (params (DecreasedMana :type "Float (double-precision)"))
  (returns (NoManaLeft :type Boolean))
  (if (not (<= (`self.CurrentMana`) 0.0))
    (set `self.CurrentMana` (- (`self.CurrentMana`) DecreasedMana))
    (`ProgressBar.SetPercent` (`/Game/Kori/UI/WB_HUD.ManaBar` (`/Game/ThirdPerson/Blueprints/BP_ThirdPersonCharacter.HUDWidget` (`self.PlayerCharacterBP`))) (/ (`self.CurrentMana`) (`self.MaxHealth`)))
    (if (<= (`self.CurrentMana`) 0.0)
      _
      (else
        (return false))))
  (return true))

(fn `DecreaseStamina`
  (params (`Stamina Depleted` :type "Float (double-precision)"))
  (returns (`No Stamina Left` :type Boolean))
  (if (not (<= (`self.CurrentStamina`) 0.0))
    (set `self.CurrentStamina` (- (`self.CurrentStamina`) `Stamina Depleted`))
    (`ProgressBar.SetPercent` (`/Game/Kori/UI/WB_HUD.StaminaBar` (`/Game/ThirdPerson/Blueprints/BP_ThirdPersonCharacter.HUDWidget` (`self.PlayerCharacterBP`))) (/ (`self.CurrentStamina`) (`self.MaxStamina`)))
    (if (<= (`self.CurrentStamina`) 0.0)
      _
      (else
        (return false))))
  (return true))

(fn `IncreaseMaxHealth`
  (params (`Added Health` :type "Float (double-precision)"))
  (set `self.MaxHealth` (+ (`self.MaxHealth`) `Added Health`))
  (`ProgressBar.SetPercent` (`/Game/Kori/UI/WB_HUD.HealthBar` (`/Game/ThirdPerson/Blueprints/BP_ThirdPersonCharacter.HUDWidget` (`self.PlayerCharacterBP`))) (/ (`self.CurrentHealth`) (`self.MaxHealth`))))

(fn `IncreaseMaxMana`
  (params (`Added Mana` :type "Float (double-precision)"))
  (set `self.MaxMana` (+ (`self.MaxMana`) `Added Mana`))
  (`ProgressBar.SetPercent` (`/Game/Kori/UI/WB_HUD.ManaBar` (`/Game/ThirdPerson/Blueprints/BP_ThirdPersonCharacter.HUDWidget` (`self.PlayerCharacterBP`))) (/ (`self.CurrentMana`) (`self.MaxMana`))))

(fn `IncreaseMaxStamina`
  (params (`Added Stamina` :type "Float (double-precision)"))
  (set `self.MaxStamina` (+ (`self.MaxStamina`) `Added Stamina`))
  (`ProgressBar.SetPercent` (`/Game/Kori/UI/WB_HUD.StaminaBar` (`/Game/ThirdPerson/Blueprints/BP_ThirdPersonCharacter.HUDWidget` (`self.PlayerCharacterBP`))) (/ (`self.CurrentStamina`) (`self.MaxStamina`))))

(fn `RecoverHealth`
  (params (`Recovering Health` :type "Float (double-precision)"))
  (set `self.CurrentHealth` (+ (`self.CurrentHealth`) `Recovering Health`))
  (if (> (`self.CurrentHealth`) (`self.MaxHealth`))
    (set `self.CurrentHealth` (`self.MaxHealth`)))
  (`ProgressBar.SetPercent` (`/Game/Kori/UI/WB_HUD.HealthBar` (`/Game/ThirdPerson/Blueprints/BP_ThirdPersonCharacter.HUDWidget` (`self.PlayerCharacterBP`))) (/ (`self.CurrentHealth`) (`self.MaxHealth`))))

(fn `RecoverMana`
  (params (`Increased Mana` :type "Float (double-precision)"))
  (set `self.CurrentMana` (+ (`self.CurrentMana`) `Increased Mana`))
  (if (>= (`self.CurrentMana`) (`self.MaxMana`))
    (set `self.CurrentMana` (`self.MaxMana`)))
  (`ProgressBar.SetPercent` (`/Game/Kori/UI/WB_HUD.ManaBar` (`/Game/ThirdPerson/Blueprints/BP_ThirdPersonCharacter.HUDWidget` (`self.PlayerCharacterBP`))) (/ (`self.CurrentMana`) (`self.MaxMana`))))

(fn `RecoverStamina`
  (params (`Recovering Stamina` :type "Float (double-precision)"))
  (set `self.CurrentStamina` (+ (`self.CurrentStamina`) `Recovering Stamina`))
  (if (> (`self.CurrentStamina`) (`self.MaxStamina`))
    (set `self.CurrentStamina` (`self.MaxStamina`)))
  (`ProgressBar.SetPercent` (`/Game/Kori/UI/WB_HUD.StaminaBar` (`/Game/ThirdPerson/Blueprints/BP_ThirdPersonCharacter.HUDWidget` (`self.PlayerCharacterBP`))) (/ (`self.CurrentStamina`) (`self.MaxStamina`))))